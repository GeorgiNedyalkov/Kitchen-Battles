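; Short-lived destructible debris actor for a dead cucumber, built on a Geometry Collection, that destroys itself a few seconds after BeginPlay.
; When BP_Veggiebond overlaps the collection, it spawns BP_WalkOverDebris_FF at that character's capsule location.
; A DoOnce gate limits this to one spawn until an end overlap from BP_Veggiebond resets it.
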(event `self.ReceiveBeginPlay`
  (`KismetSystemLibrary.Delay` 5.0)
  (`self.K2_DestroyActor`))

(event `self.GeometryCollection.OnComponentBeginOverlap`
  (params (OverlappedComponent :type "PrimitiveComponent Object Reference") (OtherActor :type "Actor Object Reference") (OtherComp :type "PrimitiveComponent Object Reference") (OtherBodyIndex :type Integer) (bFromSweep :type Boolean) (SweepResult :type "HitResult Structure (by ref)"))
  (bind _asbp_veggiebond (cast `/Game/Character/BP_Veggiebond` OtherActor))
  (`/Engine/EditorBlueprintResources/StandardMacros.DoOnce` false :!label _label
    (:`Completed`
      (`|SpawnActorFromClass` "/Game/Blueprints/Misc/BP_WalkOverDebris_FF.BP_WalkOverDebris_FF_C" (`KismetMathLibrary.Conv_VectorToTransform` (`SceneComponent.K2_GetComponentLocation` (`Character.CapsuleComponent` _asbp_veggiebond))) "Undefined" "MultiplyWithRoot" null null))))

(event `self.GeometryCollection.OnComponentEndOverlap`
  (params (OverlappedComponent :type "PrimitiveComponent Object Reference") (OtherActor :type "Actor Object Reference") (OtherComp :type "PrimitiveComponent Object Reference") (OtherBodyIndex :type Integer))
  (cast `/Game/Character/BP_Veggiebond` OtherActor)
  (goto _label :!via `Reset`))

(fn `UserConstructionScript`)