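; BP_SpawnPoint is a wave mode spawn point that spawns queued enemy classes at its own transform.
; AddEnemyToQueue appends a class and spawns immediately if no enemy overlaps the CollisionBox.
; A looping timer also pops the queue front, without that overlap check.
; Spawned enemies get a destroyed-event binding, and OnEnemyDefeated reports eliminations to the BP_WaveMode game mode.
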(event `self.ReceiveBeginPlay`
  (`KismetSystemLibrary.K2_SetTimerDelegate` (delegate `TryToSpawnEnemy`) 2.0 true)
  (bind _asbp_wave_mode (cast `/Game/Blueprints/WaveMode/BP_WaveMode` (`GameplayStatics.GetGameMode`)))
  (set `self.WaveModeRef` _asbp_wave_mode))

(event `TryToSpawnEnemy`
  (`self.SpawnNewEnemy`))

(event `OnEnemyDefeated`
  (bind _asbp_wave_mode (cast `/Game/Blueprints/WaveMode/BP_WaveMode` (`GameplayStatics.GetGameMode`)))
  (`/Game/Blueprints/WaveMode/BP_WaveMode.EnemyEliminated` _asbp_wave_mode))

(fn `AddEnemyToQueue`
  (params (EnemyClass :type "/Game/Enemies/BP_Enemy_Base Class Reference"))
  (`KismetArrayLibrary.Array_Add` (`self.EnemyQueue`) EnemyClass)
  (if (not (`KismetArrayLibrary.Array_IsValidIndex` (`PrimitiveComponent.GetOverlappingActors` (`self.CollisionBox`) "/Game/Enemies/BP_Enemy_Base.BP_Enemy_Base_C")))
    (`self.SpawnNewEnemy`)))

(fn `SpawnNewEnemy`
  (returns (Success :type Boolean))
  (if (`KismetArrayLibrary.Array_IsValidIndex` (`self.EnemyQueue`))
    (bind _returnvalue (`|SpawnActorFromClass` (`|GetArrayItem` (`self.EnemyQueue`)) (`self.GetTransform`) "AdjustIfPossibleButAlwaysSpawn" "MultiplyWithRoot" null false null))
    (add `/Game/Enemies/BP_Enemy_Base.OnEnemyDestroyed` _returnvalue (`|CreateDelegate` :!event `OnEnemyDefeated`))
    (`KismetArrayLibrary.Array_Remove` (`self.EnemyQueue`))
    (return true)
    (else
      (return false))))

(fn `UserConstructionScript`)