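; AIC_EnemyBase is the base AI controller for enemies, driving them through the BT_EnemyBase behavior tree.
; On possession it runs the tree and sets the starting state to passive.
; Two functions switch behavior by writing an E_AIState enum to the blackboard: SetStateAsPassive, and SetStateAsAttacking, which also stores the attack target object for the tree to use.
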(event `self.ReceivePossess`
  (params (PossessedPawn :type "Pawn Object Reference"))
  (`self.RunBehaviorTree` "/Game/Blueprints/AI/BT_EnemyBase.BT_EnemyBase")
  (`self.SetStateAsPassive`))

(fn `SetStateAsAttacking`
  (params (AttackTarget :type "Actor Object Reference"))
  (`BlackboardComponent.SetValueAsEnum` (`self.Blackboard`) (`self.AIStateKeyName`) (enumliteral `/Game/Blueprints/Enums/E_AIState` "NewEnumerator2"))
  (`BlackboardComponent.SetValueAsObject` (`self.Blackboard`) (`self.AttackTargetKeyName`) AttackTarget))

(fn `SetStateAsPassive`
  (`BlackboardComponent.SetValueAsEnum` (`self.Blackboard`) (`self.AIStateKeyName`) (enumliteral `/Game/Blueprints/Enums/E_AIState` "NewEnumerator1")))

(fn `UserConstructionScript`)