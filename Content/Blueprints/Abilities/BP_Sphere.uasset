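; Ability actor that runs a time-dilated, multi-target blink attack for the Veggiebond player.
; An expanding sphere stuns overlapped enemies, recording them and a blink point near each.
; After expansion, a looping timer blinks the player through those points via BPCBlink, then to the sphere's initial location.
; A delayed kill step damages all recorded enemies, spawns BP_Ability_FF per enemy, restores time and destroys the actor.
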(event `self.ReceiveBeginPlay`
  ;[0 0 0] On Begin Play: Start expanding
  (bind _asbp_veggiebond (cast `/Game/Character/BP_Veggiebond` (`GameplayStatics.GetPlayerCharacter` 0)))
  (set `self.CharacterRef` _asbp_veggiebond)
  (`GameplayStatics.SetGlobalTimeDilation` (`self.Time Dilation`))
  (bind _returnvalue (`KismetSystemLibrary.K2_SetTimerDelegate` (delegate `Expand`) (`self.ExpandTime`) true))
  (set `self.ExapandTimer` _returnvalue)
  (set `self.InitialLocation` (`self.K2_GetActorLocation`)))

(event `ED_Blink End_Event`
  ;[1 1 1] Deprecated: turn around to face enemies
  (`self.SphereTraceAttack`))

(event `Expand`
  (bind (_returnvalue_location _returnvalue_rotation _returnvalue_scale) (`KismetMathLibrary.BreakTransform` (`SceneComponent.K2_GetComponentToWorld` (`self.Sphere`))))
  ;[0 0 0] On Begin Play: Start expanding
  (`SceneComponent.K2_SetWorldTransform` (`self.Sphere`) (`KismetMathLibrary.MakeTransform` _returnvalue_location _returnvalue_rotation (+ _returnvalue_scale (0.1 0.1 0.1))) false false)
  (`KismetSystemLibrary.Delay` (`self.ExpandDuration`))
  (`KismetSystemLibrary.K2_ClearAndInvalidateTimerHandle` (`self.ExapandTimer`))
  (`SceneComponent.SetVisibility` (`self.StaticMesh`) false false)
  (`self.QuickAttack`))

(event `QuickAttack`
  (bind _returnvalue (`KismetSystemLibrary.K2_SetTimerDelegate` (delegate `StartQuickAttack`) 0.2 true))
  (set `self.QuickAttackTimer` _returnvalue))

(event `SphereTraceAttack`
  (bind _returnvalue (`GameplayStatics.GetPlayerCharacter` 0))
  (bind _returnvalue_2 (`self.K2_GetActorLocation` _returnvalue))
  ;[1 1 1] Deprecated: Sphere trace attack
  (bind (_outhit _returnvalue_3) (`KismetSystemLibrary.SphereTraceSingleForObjects` _returnvalue_2 (+ _returnvalue_2 (* (`self.GetActorForwardVector` _returnvalue) 200.0)) 100.0 (`|MakeArray` "ObjectTypeQuery3" :!type "EObjectTypeQuery Enum") false (`|MakeArray` (`GameplayStatics.GetPlayerCharacter` 0) :!type "Actor Object Reference")))
  (if _returnvalue_3
    (message `/Game/Blueprints/Interfaces/I_Damageable.TakeDamage` (`.HitActor` (`GameplayStatics.BreakHitResult` _outhit)) (make `/Game/Blueprints/Structures/S_DamageInfo` (`self.DamageAmount`) "NewEnumerator3" "NewEnumerator1"))))

(event `StartQuickAttack`
  (if (`KismetArrayLibrary.Array_IsValidIndex` (`self.BlinkLocations`))
    (`self.TeleportToLocation` (`|GetArrayItem` (`self.BlinkLocations`)))
    (`KismetArrayLibrary.Array_Remove` (`self.BlinkLocations`))
    (else
      (`/Engine/EditorBlueprintResources/StandardMacros.DoOnce` false
        (:`Completed`
          (`self.TeleportToLocation` (`self.InitialLocation`))
          (`KismetSystemLibrary.K2_SetTimerDelegate` (delegate `KillEnemies`) (`self.KillTime`)))))))

(event `KillEnemies`
  (for _array_element (`self.EnemiesInRange`)
    (message `/Game/Blueprints/Interfaces/I_Damageable.TakeDamage` _array_element (make `/Game/Blueprints/Structures/S_DamageInfo` (`self.DamageAmount`) "NewEnumerator3" "NewEnumerator1"))
    (`|SpawnActorFromClass` "/Game/Blueprints/Misc/BP_Ability_FF.BP_Ability_FF_C" (`KismetMathLibrary.Conv_VectorToTransform` (`self.InitialLocation`)) "Undefined" "MultiplyWithRoot" null null))
  (`GameplayStatics.SetGlobalTimeDilation` 1.0)
  (`self.StopQuickAttack`))

(event `StopQuickAttack`
  ;[0 0 0] End attack
  (`KismetSystemLibrary.K2_ClearAndInvalidateTimerHandle` (`self.QuickAttackTimer`))
  (`self.K2_DestroyActor`))

(event `self.Sphere.OnComponentBeginOverlap`
  (params (OverlappedComponent :type "PrimitiveComponent Object Reference") (OtherActor :type "Actor Object Reference") (OtherComp :type "PrimitiveComponent Object Reference") (OtherBodyIndex :type Integer) (bFromSweep :type Boolean) (SweepResult :type "HitResult Structure (by ref)"))
  ;[0 0 0] On Begin Overlap: Get enemies and enemy locations in range
  (if (!= OtherActor (`GameplayStatics.GetPlayerCharacter` 0))
    (bind _asbp_enemy_base (cast `/Game/Enemies/BP_Enemy_Base` OtherActor))
    (`/Game/Enemies/BP_Enemy_Base.OnStun` _asbp_enemy_base)
    (`KismetArrayLibrary.Array_Add` (`self.EnemiesInRange`) OtherActor)
    (`KismetArrayLibrary.Array_Add` (`self.BlinkLocations`) (+ (`self.K2_GetActorLocation` OtherActor) (* (`self.GetActorForwardVector` OtherActor) (120.0 0.0 0.0))))))

(fn `TeleportToLocation`
  (params (BlinkLocation :type "Vector Structure"))
  (bind _characterref (`self.CharacterRef`))
  (bind _bpc_blink (`/Game/Character/BP_Veggiebond.BPC_Blink` _characterref))
  (`KismetSystemLibrary.PrintString` "Teleporting")
  (set `/Game/Blueprints/Components/BPC_Blink.Old Location` (`SceneComponent.K2_GetComponentLocation` (`Character.CapsuleComponent` _characterref)) _bpc_blink)
  (set `/Game/Blueprints/Components/BPC_Blink.Blink Location` BlinkLocation _bpc_blink)
  (`/Game/Blueprints/Components/BPC_Blink.Event Blink Start` _bpc_blink))

(fn `UserConstructionScript`)