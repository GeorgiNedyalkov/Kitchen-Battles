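; Actor component that gives a Character a blink: a short delayed teleport along the last movement input.
; BlinkTrace steps back from maximum distance by capsule-sized increments, using sphere, line and capsule traces plus Blink_Pass/Blink_Block tags to find a clear, grounded spot, falling back to the current location.
; Blinking hides the mesh, disables input and spawns tinted Niagara effects, then a timer moves the capsule and restores both, with dispatchers at start and end.
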(event `self.ReceiveBeginPlay`
  (`|ExecutionSequence`
    (:`then_0`
      (bind _ascharacter (cast `Character` (`self.GetOwner`)))
      (bind _output_get (set `self.As Character` _ascharacter))
      (set `self.SK_Mesh` (`Character.Mesh` _output_get))
      (bind (_outradius _outhalfheight) (`CapsuleComponent.GetScaledCapsuleSize` (`Character.CapsuleComponent` _ascharacter)))
      (set `self.Default Capsule Radius` _outradius)
      (set `self.Default Capsule Half Height` _outhalfheight)
      (`self.Update Blink Values` (`self.Blink Distance`)))))

(event `Event Blink Start`
  ;[0.002428 0.002428 0.002428] Blink Logic
  (`self.ED_Blink Start`)
  (`SceneComponent.SetVisibility` (`self.SK_Mesh`) false true)
  (`Actor.DisableInput` (`self.As Character`) (`GameplayStatics.GetPlayerController` 0))
  (bind _returnvalue (`NiagaraFunctionLibrary.SpawnSystemAtLocation` (`self.FX Start`) (`self.Old Location`)))
  (`FXSystemComponent.SetColorParameter` _returnvalue "Color 1" (`self.Blink Color`))
  (bind _returnvalue_2 (`NiagaraFunctionLibrary.SpawnSystemAtLocation` (`self.FX Middle`) (`self.Blink Location`)))
  ;;[0.95 1 0.2083] Connecting/moving 'Set World Location' before 'Set Timer by Event' will make the Blink feel more instantaneous, but keeping it before 'Spawn System at Location' gives it a slight delay feel, as if it's being charged, which also compliments the visuals, imo
  (bind _output_get (set `self.NS_BlinkMiddle_Reff` _returnvalue_2))
  (`FXSystemComponent.SetColorParameter` _output_get "Color 1" (`self.Blink Color`))
  (bind _returnvalue_3 (`KismetSystemLibrary.K2_SetTimerDelegate` (delegate `Event Blink End`) (`self.Blink Delay`)))
  (set `self.Blink Timer` _returnvalue_3))

(event `Event Blink End`
  ;[0.002428 0.002428 0.002428] Blink Logic
  ;;[0.95 1 0.2083] Connecting/moving 'Set World Location' before 'Set Timer by Event' will make the Blink feel more instantaneous, but keeping it before 'Spawn System at Location' gives it a slight delay feel, as if it's being charged, which also compliments the visuals, imo
  (`SceneComponent.K2_SetWorldLocation` (`Character.CapsuleComponent` (`self.As Character`)) (`self.Blink Location`) false true)
  (bind _returnvalue (`NiagaraFunctionLibrary.SpawnSystemAtLocation` (`self.FX End`) (`SceneComponent.K2_GetComponentLocation` (`Character.CapsuleComponent` (`self.As Character`)))))
  (`FXSystemComponent.SetVectorParameter` _returnvalue "BeamEndLocation" (`self.Old Location`))
  (`FXSystemComponent.SetColorParameter` _returnvalue "Color 1" (`self.Blink Color`))
  (`self.Deactivate` (`self.NS_BlinkMiddle_Reff`))
  (`SceneComponent.SetVisibility` (`self.SK_Mesh`) true true)
  (`Actor.EnableInput` (`self.As Character`) (`GameplayStatics.GetPlayerController` 0))
  (set `self.Is Blinking?` false)
  (`self.ED_Blink End`))

(event `Event Blink Trace`
  (bind _as_character (`self.As Character`))
  (bind _returnvalue (`SceneComponent.K2_GetComponentLocation` (`Character.CapsuleComponent` _as_character)))
  (for _ (range (+ (`self.Last Index`) 1)) :!label _label
    (set `self.Old Location` _returnvalue)
    (bind (_outhit _returnvalue_2) (`KismetSystemLibrary.SphereTraceSingle` :`Start` (+ _returnvalue (0.0 0.0 20.0)) :`End` (+ _returnvalue (* (`KismetMathLibrary.Normal` (`PawnMovementComponent.GetLastInputVector` (`Character.CharacterMovement` _as_character))) (`self.Blink Distance (Temp)`))) :`Radius` 20.0 :`TraceChannel` "TraceTypeQuery1" :`DrawDebugType` (`self.Draw Debug Type`) :`DrawTime` 1.0))
    (if _returnvalue_2
      (bind (_bblockinghit _binitialoverlap _time _distance _location _impactpoint _normal _impactnormal _physmat _hitactor _hitcomponent _hitbonename _bonename _hititem _elementindex _faceindex _tracestart _traceend) (`GameplayStatics.BreakHitResult` _outhit))
      (if (`Actor.ActorHasTag` _hitactor "Blink_Pass")
        (bind (_outhit_2 _returnvalue_3) (`KismetSystemLibrary.LineTraceSingle` :`Start` (+ _traceend (0.0 0.0 100.0)) :`End` (+ _traceend (0.0 0.0 -500.0)) :`TraceChannel` "TraceTypeQuery1" :`DrawDebugType` (`self.Draw Debug Type`) :`DrawTime` 1.0 :!label _label_2))
        (if _returnvalue_3
          (bind (_bblockinghit_2 _binitialoverlap_2 _time_2 _distance_2 _location_2 _impactpoint_2 _normal_2 _impactnormal_2 _physmat_2 _hitactor_2) (`GameplayStatics.BreakHitResult` _outhit_2))
          (if (`Actor.ActorHasTag` _hitactor_2 "Blink_Block")
            (`self.Update Blink Distance (Temp)` :!label _label_3)
            (else
              (bind _returnvalue_4 (+ _location_2 (* _normal_2 100.0)))
              (bind (_outhit_3 _returnvalue_5) (`KismetSystemLibrary.CapsuleTraceSingle` :`Start` _returnvalue_4 :`End` _returnvalue_4 :`Radius` (* (`self.Default Capsule Radius`) 1.2) :`HalfHeight` (`self.Default Capsule Half Height`) :`TraceChannel` "TraceTypeQuery1" :`DrawDebugType` (`self.Draw Debug Type`) :`DrawTime` 1.0))
              (if _returnvalue_5
                (`self.Update Blink Distance (Temp)`)
                (else
                  (set `self.Blink Location` (`.TraceEnd` (`GameplayStatics.BreakHitResult` _outhit_3)))
                  (`self.Event Break Blink Loop`)))))
          (else
            (goto _label_3)))
        (else
          (`self.Update Blink Distance (Temp)`)))
      (else
        (goto _label_2))))
  (set `self.Blink Distance (Temp)` (`self.Blink Distance`))
  (if (not (`self.Is Blinking?`))
    (set `self.Blink Location` (`SceneComponent.K2_GetComponentLocation` (`Character.CapsuleComponent` (`self.As Character`))))
    (set `self.Is Blinking?` true)
    (`self.Event Blink Start`)))

(event `Event Break Blink Loop`
  (if (not (`self.Is Blinking?`))
    (set `self.Is Blinking?` true)
    (`self.Event Blink Start`)
    (goto _label :!via `Break`)))

(fn `Capsule Diameter`
  (returns (ReturnValue :type "Float (double-precision)"))
  (return (* (`self.Default Capsule Radius`) 2.4)))

(fn `Update Blink Values`
  (params (`Blink Distance (Temp)` :type "Float (single-precision)"))
  (set `self.Blink Distance (Temp)` `Blink Distance (Temp)`)
  (set `self.Last Index` (`KismetMathLibrary.FTrunc` (/ `Blink Distance (Temp)` (`self.Capsule Diameter`)))))