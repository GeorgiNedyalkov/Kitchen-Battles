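; Actor component that gives the BP_Veggiebond character physical animation on its upper skeleton, named for physical hit reactions.
; On BeginPlay it adds a PhysicalAnimationComponent to the owner and binds it to the character's mesh.
; TogglePhysicalAnimation simulates bodies below the Hips bone, applies the "Strong" profile and half-blends physics with animation.
; Despite its name, the toggle only switches physics on, with no path to disable it.
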(event `self.ReceiveBeginPlay`
  (bind _returnvalue (`|AddComponentByClass` (`self.GetOwner`) "/Script/Engine.PhysicalAnimationComponent"))
  (bind _output_get (set `self.PhysicalAnimComponent` _returnvalue))
  (bind _asbp_veggiebond (cast `/Game/MC_Tests/BP_Veggiebond` (`self.GetOwner`)))
  (bind _mesh (`Character.Mesh` _asbp_veggiebond))
  (`PhysicalAnimationComponent.SetSkeletalMeshComponent` _output_get _mesh)
  (set `self.Mesh` _mesh))

(event `TogglePhysicalAnimation`
  (`SkeletalMeshComponent.SetAllBodiesBelowSimulatePhysics` (`self.Mesh`) "Hips" true false)
  (`PhysicalAnimationComponent.ApplyPhysicalAnimationProfileBelow` (`self.PhysicalAnimComponent`) "Hips" "Strong" false false)
  (`SkeletalMeshComponent.SetAllBodiesBelowPhysicsBlendWeight` (`self.Mesh`) "Hips" 0.5 false true))