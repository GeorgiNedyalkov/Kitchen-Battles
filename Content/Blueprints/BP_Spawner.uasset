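; Enemy spawner actor that holds a queue of enemy classes and spawns them one at a time at its own transform.
; A looping timer pops the queue, and newly queued enemies trigger an immediate spawn attempt when no enemy overlaps its collision sphere.
; It binds to each enemy's destroyed event, can report defeats to the game mode, and updates its IsOn flag from the wave count at wave end.
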(event `self.ReceiveBeginPlay`
  (`KismetSystemLibrary.K2_SetTimerDelegate` (delegate `TryToSpawnEnemy`) 2.0 true)
  (bind _asbp_third_person_game_mode (cast `/Game/Blueprints/BP_ThirdPersonGameMode` (`GameplayStatics.GetGameMode`)))
  (bind _output_get (set `self.GameMode` _asbp_third_person_game_mode))
  (add `/Game/Blueprints/BP_ThirdPersonGameMode.OnEndWave` _output_get (delegate `OnEndWave`)))

(event `OnEndWave`
  (set `self.bIsOn` (>= (`self.RoundActivated`) (+ (`/Game/Blueprints/BP_ThirdPersonGameMode.WaveCount` (`self.GameMode`)) 1))))

(event `TryToSpawnEnemy`
  (`self.SpawnEnemy`))

(event `OnEnemyDefeated`
  (bind _asbp_third_person_game_mode (cast `/Game/Blueprints/BP_ThirdPersonGameMode` (`GameplayStatics.GetGameMode`)))
  (`/Game/Blueprints/BP_ThirdPersonGameMode.OnEnemyDefeated` _asbp_third_person_game_mode))

(fn `AddEnemyToQueue`
  (params (EnemyClass :type "/Game/Enemies/BP_Enemy Class Reference"))
  (`KismetArrayLibrary.Array_Add` (`self.EnemyQueue`) EnemyClass)
  (if (not (`KismetArrayLibrary.Array_IsValidIndex` (`PrimitiveComponent.GetOverlappingActors` (`self.CollisionSphere`) "/Game/Enemies/BP_Enemy.BP_Enemy_C")))
    (`self.SpawnEnemy`)))

(fn `SpawnEnemy`
  (returns (bSuccess :type Boolean))
  (if (`KismetArrayLibrary.Array_IsValidIndex` (`self.EnemyQueue`))
    (bind _returnvalue (`|SpawnActorFromClass` (`|GetArrayItem` (`self.EnemyQueue`)) (`self.GetTransform`) "AdjustIfPossibleButAlwaysSpawn" "MultiplyWithRoot" null null))
    (add `/Game/Enemies/BP_Enemy.OnEnemyDestroyed` _returnvalue (`|CreateDelegate` :!event `OnEnemyDefeated`))
    (`KismetArrayLibrary.Array_Remove` (`self.EnemyQueue`))
    (return true)
    (else
      (return false))))

(fn `UserConstructionScript`)