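; Interaction component that tracks whether its owning actor can be interacted with and whether it is activated.
; Enable and disable events set Interactable and broadcast OnToggleInteractivity, while starting (only when interactable) and stopping interaction set Activated and broadcast OnInteract.
; An orientation check compares player pawn and owner forward vectors by dot product, enabling interactivity only when they are not closely aligned.
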(event `EnableInteractivity`
  (set `self.bInteractable` true)
  (`self.OnToggleInteractivity`))

(event `DisableInteractivity`
  (set `self.bInteractable` false)
  (`self.OnToggleInteractivity`))

(event `StartInteraction`
  (if (`self.bInteractable`)
    (set `self.bActivated` true)
    (`self.OnInteract` true)))

(event `StopInteraction`
  (set `self.bActivated` false)
  (`self.OnInteract` false))

(event `StartCharacterOrientationCheck`
  (if (<= (`KismetMathLibrary.Dot_VectorVector` (`Actor.GetActorForwardVector` (`GameplayStatics.GetPlayerPawn` 0)) (`Actor.GetActorForwardVector` (`self.GetOwner`))) 0.5)
    (`self.EnableInteractivity`)
    (else
      (`self.DisableInteractivity`))))