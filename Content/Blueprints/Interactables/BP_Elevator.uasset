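; BP_Elevator is an elevator actor that moves its Cube component between a start and an end position.
; Two custom events play or reverse the ElevatorHeight timeline, whose curve drives a lerp of the cube's relative location without sweep.
; An IsAtEndPosition flag gates each direction and flips when the timeline finishes.
; Nothing in this Blueprint calls the events, and its default event nodes are disabled.
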(event `MoveToEndLocation`
  (if (not (`self.bIsAtEndPosition`))
    (bind (_direction _elevatormovement) (`Timeline|ElevatorHeight` :!label _label)
      (:`Update`
        (`SceneComponent.K2_SetRelativeLocation` (`self.Cube`) (`KismetMathLibrary.VLerp` (`self.StartPosition`) (`self.EndPosition`) _elevatormovement) false false))
      (:`Finished`
        (set `self.bIsAtEndPosition` (not (`self.bIsAtEndPosition`)))))))

(event `MoveToStartLocation`
  (if (`self.bIsAtEndPosition`)
    (goto _label :!via `Reverse`)))

(fn `UserConstructionScript`)