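; BP_Button is an interactable push button that moves and glows when used.
; BPInteractionComponent's interact event plays a timeline that offsets the button mesh on all three axes and drives the Emissive parameter of a dynamic material created in the construction script.
; HintText is shown on interactivity toggle and on sphere overlap begin; overlap end also sets it visible, so nothing here hides it.
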(event `self.ReceiveBeginPlay`
  (bind _bp_interaction_component (`self.BP_Interaction_Component`))
  (add `/Game/Blueprints/Interactables/BP_Interaction_Component.OnInteract` _bp_interaction_component (delegate `StartInteraction`))
  (add `/Game/Blueprints/Interactables/BP_Interaction_Component.OnToggleInteractivity` _bp_interaction_component (delegate `DisplayHint`)))

(event `StartInteraction`
  (params (On :type Boolean))
  (`self.PressButton`))

(event `DisplayHint`
  (`SceneComponent.SetVisibility` (`self.HintText`) true false))

(event `PressButton`
  (bind (_direction _buttonmovement) (`Timeline|Timeline`)
    (:`Update`
      (bind _returnvalue (* _buttonmovement -10.0))
      (`SceneComponent.K2_SetRelativeLocation` (`self.Button`) (`KismetMathLibrary.MakeVector` _returnvalue _returnvalue _returnvalue) false false)
      (`MaterialInstanceDynamic.SetScalarParameterValue` (`self.Material`) "Emissive" (* _buttonmovement 5.0)))))

(event `self.Sphere.OnComponentBeginOverlap`
  (params (OverlappedComponent :type "PrimitiveComponent Object Reference") (OtherActor :type "Actor Object Reference") (OtherComp :type "PrimitiveComponent Object Reference") (OtherBodyIndex :type Integer) (bFromSweep :type Boolean) (SweepResult :type "HitResult Structure (by ref)"))
  (`self.DisplayHint`))

(event `self.Sphere.OnComponentEndOverlap`
  (params (OverlappedComponent :type "PrimitiveComponent Object Reference") (OtherActor :type "Actor Object Reference") (OtherComp :type "PrimitiveComponent Object Reference") (OtherBodyIndex :type Integer))
  (`SceneComponent.SetVisibility` (`self.HintText`) true false))

(fn `UserConstructionScript`
  (bind _returnvalue (`PrimitiveComponent.CreateDynamicMaterialInstance` (`self.Button`) 0 "/Engine/MapTemplates/Materials/BasicAsset03.BasicAsset03" "None"))
  (set `self.Material` _returnvalue))