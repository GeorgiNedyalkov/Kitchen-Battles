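; Base enemy character that exposes health, damage, patrol route and movement speed functions, leaving Attack and face expression as empty stubs.
; BPCDamageSystem owns health, damage and healing, with its death and damage-response events bound in the construction script.
; An overhead health bar widget references the enemy, and hit reactions play a montage.
; Death enables mesh physics, removes the bar, destroys the actor and calls OnEnemyDestroyed.
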(event `self.ReceiveBeginPlay`
  ;[0.002428 0.002428 0.002428] Event Begin Play
  (bind _returnvalue (`|CreateWidget` "/Game/UI/W_HealthBar_Overhead.W_HealthBar_Overhead_C" null self))
  (`WidgetComponent.SetWidget` (`self.Healthbar`) _returnvalue)
  (message `/Game/Blueprints/Interfaces/I_Damageable.GetHealthPercentage` self))

(event `DamageResponse`
  (params (DamageResponse :type "/Game/Blueprints/Enums/E_DamageResponse Enum" :default "NewEnumerator0"))
  ;[0.002428 0.002428 0.002428] Event on Hit Response
  (`self.PlayAnimMontage` (select `/Game/Blueprints/Enums/E_DamageResponse` DamageResponse :`NewEnumerator1` "/Game/HitImpact_Montage.HitImpact_Montage" :!type "AnimMontage Object Reference"))
  (message `/Game/Blueprints/Interfaces/I_Damageable.GetHealthPercentage` self))

(event `Death`
  (bind _mesh (`self.Mesh`))
  ;[0.002428 0.002428 0.002428] Event On Death
  (`PrimitiveComponent.SetSimulatePhysics` _mesh true)
  (`PrimitiveComponent.SetCollisionEnabled` _mesh "QueryAndPhysics")
  (message `/Game/Blueprints/Interfaces/I_Damageable.GetHealthPercentage` self)
  (`ActorComponent.K2_DestroyComponent` (`self.Healthbar`))
  (`self.K2_DestroyActor`)
  (`self.OnEnemyDestroyed`))

(event `Attack`)

(fn `GetCurrentHealth`
  (returns (CurrentHealth :type "Float (double-precision)"))
  (return (`/Game/Blueprints/Components/BPC_DamageSystem.Health` (`self.BPC_DamageSystem`))))

(fn `GetHealthPercentage`
  (returns (HealthPercentage :type "Float (double-precision)"))
  (bind _bpc_damagesystem (`self.BPC_DamageSystem`))
  (bind _returnvalue (/ (`/Game/Blueprints/Components/BPC_DamageSystem.Health` _bpc_damagesystem) (`/Game/Blueprints/Components/BPC_DamageSystem.MaxHealth` _bpc_damagesystem)))
  (`self.OnHealthUpdate` _returnvalue)
  (return _returnvalue))

(fn `GetMaxHealth`
  (returns (MaxHealth :type "Float (double-precision)"))
  (return (`/Game/Blueprints/Components/BPC_DamageSystem.MaxHealth` (`self.BPC_DamageSystem`))))

(fn `GetPatrolRoute`
  (returns (PatrolRoute :type "/Game/Blueprints/BP_PatrolRoute Object Reference"))
  (return (`self.PatrolRoute`)))

(fn `Heal`
  (params (Amount :type "Float (double-precision)"))
  (returns (NewHealth :type "Float (double-precision)"))
  (bind _newhealth (`/Game/Blueprints/Components/BPC_DamageSystem.Heal` (`self.BPC_DamageSystem`) Amount))
  (return _newhealth))

(fn `SetFaceExpression`
  (params (State :type "/Game/Blueprints/Enums/E_AIState Enum" :default "NewEnumerator0")))

(fn `SetMovementSpeed`
  (params (SpeedState :type "/Game/Blueprints/Enums/E_MovementSpeed Enum" :default "NewEnumerator0"))
  (returns (Speed :type "Float (double-precision)"))
  (bind _output_get (set `CharacterMovementComponent.MaxWalkSpeed` (select `/Game/Blueprints/Enums/E_MovementSpeed` SpeedState :`NewEnumerator0` 100.0 :`NewEnumerator1` 150.0 :`NewEnumerator2` 200.0 :`NewEnumerator3` 300.0 :!type "Float (single-precision)") (`self.CharacterMovement`)))
  (return _output_get))

(fn `TakeDamage`
  (params (DamageInfo :type "/Game/Blueprints/Structures/S_DamageInfo Structure"))
  (returns (WasDamaged :type Boolean))
  (bind _wasdamaged (`/Game/Blueprints/Components/BPC_DamageSystem.Take Damage` (`self.BPC_DamageSystem`) DamageInfo))
  (return _wasdamaged))

(fn `UserConstructionScript`
  (bind _bpc_damagesystem (`self.BPC_DamageSystem`))
  (add `/Game/Blueprints/Components/BPC_DamageSystem.OnDeath` _bpc_damagesystem (`|CreateDelegate` :!event `Death`))
  (add `/Game/Blueprints/Components/BPC_DamageSystem.OnDamageResponse` _bpc_damagesystem (`|CreateDelegate` :!event `DamageResponse`)))