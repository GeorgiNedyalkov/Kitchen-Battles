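; Base area-of-effect Blueprint for effects that act over time, extending its parent's Trigger event.
; On Trigger it runs the parent logic, then starts two looping timers, one paced by SpawnInterval and the other by Duration.
; The Duration timer also loops rather than firing once, and the file does not show what either timer's bound event does.
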(event `self.Trigger`
  (`parent.Trigger`)
  (`|ExecutionSequence`
    (:`then_0`
      (`KismetSystemLibrary.K2_SetTimerDelegate` (`|CreateDelegate` :!event `SpawnAOESphere`) (`self.SpawnInterval`) true))
    (:`then_1`
      (`KismetSystemLibrary.K2_SetTimerDelegate` (`|CreateDelegate` :!event `K2_DestroyActor`) (`self.Duration`) true))))

(fn `UserConstructionScript`
  (`parent.UserConstructionScript`))