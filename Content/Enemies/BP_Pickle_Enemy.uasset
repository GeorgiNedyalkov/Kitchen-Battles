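; BP_Pickle_Enemy is an enemy that fires projectiles at a regular interval.
; On BeginPlay a looping timer set by ShootFrequency calls Shoot, which spawns ProjectileClass at the ShootPoint transform.
; Each projectile receives the enemy as owner and its Target as a spawn parameter.
; The construction script only reassigns Target to itself when valid, so it has no apparent effect.
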(event `self.ReceiveBeginPlay`
  (`KismetSystemLibrary.K2_SetTimerDelegate` (delegate `Shoot`) (`self.ShootFrequency`) true))

(event `Shoot`
  (`|SpawnActorFromClass` (`self.ProjectileClass`) (`SceneComponent.K2_GetComponentToWorld` (`self.ShootPoint`)) "Undefined" "MultiplyWithRoot" self 500.0 0.0 false 0.0 (`self.Target`) null))

(fn `UserConstructionScript`
  (bind _target (`self.Target`)
    (:`then`
      (set `self.Target` _target))
    (:`else`)))