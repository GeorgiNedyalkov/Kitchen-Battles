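; Broccoli enemy that telekinetically lifts BP_Throwable actors in the level and hurls them at the player.
; On BeginPlay it gathers all throwables, then a timeline raises the first one toward a lift height.
; It then enables physics and applies an impulse toward the player.
; After a delay it disables physics, drops that entry and repeats, refilling the list when empty; the random-pick helper is unused.
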(event `self.ReceiveBeginPlay`
  (`parent.ReceiveBeginPlay`)
  (bind _outactors (`GameplayStatics.GetAllActorsOfClass` "/Game/Blueprints/Throwables/BP_Throwable.BP_Throwable_C"))
  (bind _output_get (set `self.ThrowableObjects` _outactors))
  (if (`KismetArrayLibrary.Array_IsEmpty` _output_get)
    (`KismetSystemLibrary.PrintString` "Brocolli: No objects in scene")
    (else
      (`self.LiftObject`))))

(event `LiftObject`
  (bind _objecttothrow (`self.ObjectToThrow`))
  (bind (_returnvalue_x _returnvalue_y _returnvalue_z) (`KismetMathLibrary.BreakVector` (`self.K2_GetActorLocation` _objecttothrow)))
  ;[0.002428 0.002428 0.002428] Lift Object
  (bind _objecttothrow_2 (`self.GetObjectToThrow`))
  (set `self.ObjectToThrow` _objecttothrow_2)
  (bind (_direction _alpha) (`Timeline|Timeline_0` :!via `PlayFromStart`)
    (:`Update`
      (`self.K2_SetActorRelativeLocation` _objecttothrow (`KismetMathLibrary.MakeVector` _returnvalue_x _returnvalue_y (`KismetMathLibrary.Lerp` _returnvalue_z (`self.LiftHeight`) _alpha)) false false))
    (:`Finished`
      (`self.ThrowObject`))))

(event `ThrowObject`
  (bind _objecttothrow (`self.ObjectToThrow`))
  (bind _staticmesh (`/Game/Blueprints/Throwables/BP_Throwable.StaticMesh` _objecttothrow))
  ;[0.002428 0.002428 0.002428] Throw Object
  (`PrimitiveComponent.SetSimulatePhysics` _staticmesh true)
  (`PrimitiveComponent.AddImpulse` _staticmesh (* (`KismetMathLibrary.Normal` (- (`self.K2_GetActorLocation` (`GameplayStatics.GetPlayerCharacter` 0)) (`self.K2_GetActorLocation` _objecttothrow))) (* (`self.ThrowVelocity`) 1000.0)) "None" false)
  (`KismetSystemLibrary.Delay` 3.0)
  (`self.NextThrow`))

(event `NextThrow`
  ;[0.002428 0.002428 0.002428] Throw Object
  (`PrimitiveComponent.SetSimulatePhysics` (`/Game/Blueprints/Throwables/BP_Throwable.StaticMesh` (`self.ObjectToThrow`)) false)
  (set `self.ObjectToThrow` null)
  (`KismetArrayLibrary.Array_Remove` (`self.ThrowableObjects`))
  (`self.LiftObject`))

(fn `GetObjectToThrow`
  (returns (ObjectToThrow :type "/Game/Blueprints/Throwables/BP_Throwable Object Reference"))
  (if (`KismetArrayLibrary.Array_IsValidIndex` (`self.ThrowableObjects`))
    (return (`|GetArrayItem` (`self.ThrowableObjects`)))
    (else
      (`KismetSystemLibrary.PrintString` "Starting again")
      (bind _outactors (`GameplayStatics.GetAllActorsOfClass` "/Game/Blueprints/Throwables/BP_Throwable.BP_Throwable_C"))
      (bind _output_get (set `self.ThrowableObjects` _outactors))
      (return (`|GetArrayItem` _output_get)))))

(fn `GetRandomObjectToThrow`
  (returns (OutItem :type "/Game/Blueprints/Throwables/BP_Throwable Object Reference"))
  (return (`KismetArrayLibrary.Array_Random` (`self.ThrowableObjects`))))

(fn `UserConstructionScript`
  (`parent.UserConstructionScript`))