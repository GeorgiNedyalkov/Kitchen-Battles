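; Ranged cucumber enemy that targets the player character with spawned projectiles.
; Attack fires a vertical column of low-damage projectiles from ShootPoint; single, delayed triple and horizontal-row shot patterns are also defined but not used by Attack.
; On death it spawns a destructible cucumber actor in its place and destroys itself.
; SetFaceExpression swaps the face decal material by AI state.
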(event `self.ReceiveBeginPlay`
  ;[0.002428 0.002428 0.002428] Event Begin Play
  (`parent.ReceiveBeginPlay`)
  (set `self.AttackTarget` (`GameplayStatics.GetPlayerCharacter` 0))
  (set `self.bIsRanged?` true))

(event `Triple Shot`
  ;[0 0 0] Tripple Shot Attack
  (`self.Shoot`)
  (`KismetSystemLibrary.Delay` 2.0)
  (`self.Shoot`)
  (`KismetSystemLibrary.Delay` 2.0)
  (`self.Shoot`))

(event `Single Shot`
  ;[0 0 0] Single Shot Attack
  (`self.Shoot`))

(event `/Game/Blueprints/Interfaces/I_EnemyAI.Attack`
  ;[0.002428 0.002428 0.002428] Event Attack
  (`self.VerticalShot`))

(event `HorizontalShot`
  (bind (_returnvalue_x _returnvalue_y _returnvalue_z) (`KismetMathLibrary.BreakVector` (`SceneComponent.K2_GetComponentLocation` (`self.ShootPoint`))))
  ;[0 0 0] Horizontal Shot
  (for _index (range 6)
    (`|SpawnActorFromClass` (`self.Projectile`) (`KismetMathLibrary.MakeTransform` (`KismetMathLibrary.MakeVector` _returnvalue_x (+ (* _index 50) _returnvalue_y) _returnvalue_z) (`self.K2_GetActorRotation`)) "DontSpawnIfColliding" "MultiplyWithRoot" self false 0.0 false (`self.AttackTarget`) 1000.0 null null 1.0 null)))

(event `Shoot`
  ;[0.002428 0.002428 0.002428] Shoot
  (`|SpawnActorFromClass` (`self.Projectile`) (`KismetMathLibrary.MakeTransform` (`SceneComponent.K2_GetComponentLocation` (`self.ShootPoint`)) (`self.K2_GetActorRotation`)) "DontSpawnIfColliding" "MultiplyWithRoot" self false 0.0 false (`self.AttackTarget`) 1000.0 null null 50.0 null))

(event `VerticalShot`
  (bind (_returnvalue_x _returnvalue_y _returnvalue_z) (`KismetMathLibrary.BreakVector` (`SceneComponent.K2_GetComponentLocation` (`self.ShootPoint`))))
  ;[0 0 0] Vertical Shot
  (for _index (range 4)
    (`|SpawnActorFromClass` (`self.Projectile`) (`KismetMathLibrary.MakeTransform` (`KismetMathLibrary.MakeVector` _returnvalue_x _returnvalue_y (- _returnvalue_z (* _index 50))) (`self.K2_GetActorRotation`)) "DontSpawnIfColliding" "MultiplyWithRoot" self false 0.0 false (`self.AttackTarget`) 1000.0 null null 1.0 null)))

(event `self.Death`
  (bind _returnvalue_location (`KismetMathLibrary.BreakTransform` (`SceneComponent.K2_GetComponentToWorld` (`self.Cucumber`))))
  ;[0 0 0] On death, replace and destroy Actor with Destructible version.
  (`parent.Death`)
  (`|SpawnActorFromClass` "/Game/Destructibles/BP_Cucumber_OnDeath.BP_Cucumber_OnDeath_C" (`KismetMathLibrary.MakeTransform` _returnvalue_location) "AlwaysSpawn" "MultiplyWithRoot" null null)
  (`self.K2_DestroyActor`))

(fn `SetFaceExpression`
  (params (State :type "/Game/Blueprints/Enums/E_AIState Enum" :default "NewEnumerator0"))
  (returns (FaceExpression :type "DecalComponent Object Reference"))
  (bind _face (`self.Face`))
  (`DecalComponent.SetDecalMaterial` _face (select `/Game/Blueprints/Enums/E_AIState` State :`NewEnumerator0` "/Game/Enemies/Faces/MI_EnemyFace_1.MI_EnemyFace_1" :`NewEnumerator1` "/Game/Enemies/Faces/MI_EnemyFace_2.MI_EnemyFace_2" :`NewEnumerator2` "/Game/Enemies/Faces/MI_EnemyFace_3.MI_EnemyFace_3" :`NewEnumerator3` "/Game/Enemies/Faces/MI_EnemyFace_4.MI_EnemyFace_4" :!type "MaterialInterface Object Reference"))
  (return _face))

(fn `UserConstructionScript`
  (`parent.UserConstructionScript`))