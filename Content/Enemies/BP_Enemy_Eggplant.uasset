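; Eggplant enemy whose attack leaps into the air and drops an area-of-effect hit on the player's position.
; Attack launches it upward while capturing the player's location and marking it with a decal, then repositions the enemy above that spot.
; After a delay, it spawns BP_Eggplant_Drop_AOE there at zero height with the configured range.
; The AOE's finish callback removes the decal; an optional debug sphere shows the radius.
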(event `self.ReceiveBeginPlay`
  (`parent.ReceiveBeginPlay`))

(event `/Game/Blueprints/Interfaces/I_EnemyAI.Attack`
  (`KismetSystemLibrary.PrintString` "Attacking")
  (`self.LaunchCharacter` (0.0 0.0 2000.0))
  (`self.AOE attack`)
  (`KismetSystemLibrary.Delay` 1.0)
  (`self.K2_SetActorRelativeLocation` (+ (`self.DropLocation`) (0.0 0.0 900.0))))

(event `AOE attack`
  (set `self.DropLocation` (`self.K2_GetActorLocation` (`GameplayStatics.GetPlayerCharacter` 0)))
  (`self.TryDrawDebugSphere`)
  (bind _returnvalue (`GameplayStatics.SpawnDecalAtLocation` "/Game/Enemies/Faces/MI_EnemyFace_3.MI_EnemyFace_3" (400.0 400.0 400.0) (`self.DropLocation`)))
  (set `self.SpawnDecal` _returnvalue)
  (`KismetSystemLibrary.Delay` (`self.AOESpawnTime`))
  (bind _returnvalue_2 (`|SpawnActorFromClass` "/Game/Blueprints/AOE/BP_Eggplant_Drop_AOE.BP_Eggplant_Drop_AOE_C" (`KismetMathLibrary.MakeTransform` (* (`self.DropLocation`) (1.0 1.0 0.0))) "Undefined" "MultiplyWithRoot" null (`self.AOERange`) null))
  (add `/Game/Blueprints/AOE/BP_Eggplant_Drop_AOE.OnFinishedAOE` _returnvalue_2 (delegate `FinishedAOE`)))

(event `FinishedAOE`
  (bind _spawndecal (`self.SpawnDecal`)
    (:`then`
      (`ActorComponent.K2_DestroyComponent` _spawndecal))
    (:`else`)))

(fn `TryDrawDebugSphere`
  (if (`self.bDrawDebugSphere`)
    (`KismetSystemLibrary.DrawDebugSphere` (`self.DropLocation`) (`self.AOERange`) 12 (struct :`R` 1.0 :`G` 1.0 :`B` 1.0 :`A` 1.0) 5.0)
    (return)
    (else
      (return))))

(fn `UserConstructionScript`
  (`parent.UserConstructionScript`))