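; Zucchini enemy Blueprint, a ranged attacker that fires projectile bursts at the player.
; On Begin Play it runs the parent logic, flags itself as ranged and sets the first player character as its attack target.
; The Attack event calls Shoot three times with short delays.
; Each Shoot spawns a projectile at the ShootPoint, facing the actor's rotation, and passes it the target and an explosion impact effect.
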(event `self.ReceiveBeginPlay`
  ;[0.002428 0.002428 0.002428] Event Begin Play
  (`parent.ReceiveBeginPlay`)
  (set `self.AttackTarget` (`GameplayStatics.GetPlayerCharacter` 0))
  (set `self.bIsRanged?` true))

(event `self.Attack`
  ;[0.002428 0.002428 0.002428] Event Attack
  (`self.Shoot`)
  (`KismetSystemLibrary.Delay` 0.2)
  (`self.Shoot`)
  (`KismetSystemLibrary.Delay` 0.2)
  (`self.Shoot`)
  (`KismetSystemLibrary.Delay` 0.2))

(event `Shoot`
  ;[0.002428 0.002428 0.002428] Shoot
  (`|SpawnActorFromClass` (`self.Projectile`) (`KismetMathLibrary.MakeTransform` (`SceneComponent.K2_GetComponentLocation` (`self.ShootPoint`)) (`self.K2_GetActorRotation`)) "Undefined" "MultiplyWithRoot" self 1000.0 0.0 false "/Game/StarterContent/Particles/P_Explosion.P_Explosion" null 0.0 (`self.AttackTarget`) null))

(fn `UserConstructionScript`
  (`parent.UserConstructionScript`))