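; Tomato enemy that attacks the player with a predictive leap.
; Attack projects the player's horizontal velocity ahead to estimate a landing point, then launches the character there along a suggested projectile arc.
; HitBox damages the player on any overlap; a separate test short-range attack damages pawns via a forward sphere trace.
; GetIdealRange supplies attack and defend radii, while speed, patrol, expression and health functions are empty stubs.
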(event `self.ReceiveBeginPlay`
  (`parent.ReceiveBeginPlay`))

(event `/Game/Blueprints/Interfaces/I_EnemyAI.Attack`
  ;[0 0 0] Attack event - Set Attack Target in AIC
  (`self.JumpAttack` (`GameplayStatics.GetPlayerCharacter` 0)))

(event `self.HitBox.OnComponentBeginOverlap`
  (params (OverlappedComponent :type "PrimitiveComponent Object Reference") (OtherActor :type "Actor Object Reference") (OtherComp :type "PrimitiveComponent Object Reference") (OtherBodyIndex :type Integer) (bFromSweep :type Boolean) (SweepResult :type "HitResult Structure (by ref)"))
  (bind _returnvalue (`GameplayStatics.GetPlayerCharacter` 0))
  ;[0 0 0] Jump Attack Hit Box
  (if (== _returnvalue (`.HitActor` (`GameplayStatics.BreakHitResult` SweepResult)))
    (message `/Game/Blueprints/Interfaces/I_Damageable.TakeDamage` _returnvalue (make `/Game/Blueprints/Structures/S_DamageInfo` 20.0 "NewEnumerator3"))))

(event `JumpAttack`
  (params (AttackTarget :type "Actor Object Reference"))
  ;[0 0 0] Jump Attack
  (bind _actorlocation (`self.CalculateNextLocation` AttackTarget))
  (bind _outlaunchvelocity (`GameplayStatics.SuggestProjectileVelocity_CustomArc` (`self.K2_GetActorLocation`) (`KismetMathLibrary.MakeVector` (.x _actorlocation) (.y _actorlocation) (+ (.z _actorlocation) 100.0))))
  (`self.LaunchCharacter` _outlaunchvelocity))

(event `ShortRangeAttack`
  (bind _returnvalue (`self.K2_GetActorLocation`))
  ;[0 0 0] Test Attack
  (bind (_outhit _returnvalue_2) (`KismetSystemLibrary.SphereTraceSingleForObjects` _returnvalue (+ _returnvalue (* (`self.GetActorForwardVector`) 200.0)) 100.0 (`|MakeArray` "ObjectTypeQuery3" :!type "EObjectTypeQuery Enum")))
  (if _returnvalue_2
    (message `/Game/Blueprints/Interfaces/I_Damageable.TakeDamage` (`.HitActor` (`GameplayStatics.BreakHitResult` _outhit)) (make `/Game/Blueprints/Structures/S_DamageInfo` 20.0 "NewEnumerator3" "NewEnumerator1"))
    (else
      (`KismetSystemLibrary.PrintString` "No Hit"))))

(fn `CalculateNextLocation`
  (params (Actor :type "Actor Object Reference") (Time :type "Float (double-precision)" :default 1.0))
  (returns (ActorLocation :type "Vector Structure"))
  (locals (NewLocalVar :type "Vector Structure"))
  (return (+ (`self.K2_GetActorLocation` Actor) (* (* (`self.GetVelocity` Actor) (1.0 1.0 0.0)) Time))))

(fn `GetCurrentHealth`
  (returns (CurrentHealth :type "Float (double-precision)"))
  (return 0.0))

(fn `GetIdealRange`
  (returns (AttackRadius :type "Float (double-precision)") (DefendRadius :type "Float (double-precision)"))
  (return 200.0 400.0))

(fn `GetPatrolRoute`
  (returns (PatrolRoute :type "/Game/Enemies/AI/BP_PatrolRoute Object Reference"))
  (return null))

(fn `SetFaceExpression`
  (params (State :type "/Game/Blueprints/Enums/E_AIState Enum" :default "NewEnumerator0"))
  (returns (FaceExpression :type "DecalComponent Object Reference"))
  (return null))

(fn `SetMovementSpeed`
  (params (SpeedState :type "/Game/Blueprints/Enums/E_MovementSpeed Enum" :default "NewEnumerator0"))
  (returns (Speed :type "Float (double-precision)"))
  (return 0.0))

(fn `UserConstructionScript`
  (`parent.UserConstructionScript`))