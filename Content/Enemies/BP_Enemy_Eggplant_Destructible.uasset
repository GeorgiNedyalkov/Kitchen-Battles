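; Destructible eggplant enemy that reacts to damage and breaks apart on death, extending a parent enemy Blueprint.
; Taking damage briefly swaps the face decal material, then switches it after half a second.
; Death enables physics on the geometry collection and destroys the capsule.
; It also spawns a short-lived master field for radial force to scatter the pieces, noted as not working, with the field flag disabled.
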(event `self.ReceiveBeginPlay`
  (`parent.ReceiveBeginPlay`))

(event `self.ReceiveAnyDamage`
  (params (Damage :type "Float (single-precision)") (DamageType :type "DamageType Object Reference") (InstigatedBy :type "Controller Object Reference") (DamageCauser :type "Actor Object Reference"))
  (bind _face (`self.Face`))
  (`DecalComponent.SetDecalMaterial` _face "/Game/Enemies/Faces/MI_EnemyFace_4.MI_EnemyFace_4")
  (`KismetSystemLibrary.Delay` 0.5)
  (`DecalComponent.SetDecalMaterial` _face "/Game/Enemies/Faces/MI_EnemyFace_3.MI_EnemyFace_3"))

(event `self.Death`
  (bind _gc_eggplant (`self.GC_Eggplant`))
  ;[0.06221 1 0.2333] Enables fractured pieces by turning on physics simulation.
  (`parent.Death`)
  (`PrimitiveComponent.SetSimulatePhysics` _gc_eggplant true)
  ;[1 0.2238 0.09399] Trying to apply force so the fractured pieces go flying instead of just falling on the ground. (Not wokring)
  (bind _returnvalue (`|SpawnActorFromClass` "/Engine/EditorResources/FieldNodes/FS_MasterField.FS_MasterField_C" (`KismetMathLibrary.Conv_VectorToTransform` (`SceneComponent.K2_GetComponentLocation` _gc_eggplant)) "AlwaysSpawn" "MultiplyWithRoot" null null))
  (`self.SetLifeSpan` _returnvalue 0.5)
  (`FieldSystemComponent.ApplyRadialForce` (`FieldSystemActor.FieldSystemComponent` _returnvalue) false (0.0 0.0 0.0) 500.0)
  (`ActorComponent.K2_DestroyComponent` (`self.CapsuleComponent`)))

(fn `UserConstructionScript`
  (`parent.UserConstructionScript`))