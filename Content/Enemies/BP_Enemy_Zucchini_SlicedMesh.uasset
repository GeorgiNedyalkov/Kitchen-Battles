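; Zucchini enemy (sliced mesh) Blueprint that attacks pawns in front of it and uses BPCDamageSystem for health.
; A looping timer from BeginPlay runs a debug-drawn forward sphere trace and sends damage to the hit actor.
; Construction binds component death and damage-response delegates, with Death ragdolling the mesh and AnyDamage playing a hit montage.
; Health getters read the component, but TakeDamage is a stub returning false.
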(event `self.ReceiveBeginPlay`
  (`KismetSystemLibrary.K2_SetTimerDelegate` (delegate `Attack`) 2.0 true)
  ;[1 1 1] Health Component
  (`KismetSystemLibrary.PrintString` "Add Health Component to Enemy"))

(event `Attack`
  (bind _returnvalue (`self.K2_GetActorLocation`))
  (bind (_outhit _returnvalue_2) (`KismetSystemLibrary.SphereTraceSingleForObjects` :`Start` _returnvalue :`End` (+ _returnvalue (* (`self.GetActorForwardVector`) 100.0)) :`Radius` 20.0 :`ObjectTypes` (`|MakeArray` "ObjectTypeQuery3" :!type "EObjectTypeQuery Enum") :`DrawDebugType` "ForDuration" :`DrawTime` 1.0))
  (if _returnvalue_2
    (message `/Game/Blueprints/Interfaces/I_Damageable.TakeDamage` (`.HitActor` (`GameplayStatics.BreakHitResult` _outhit)) (make `/Game/Blueprints/Structures/S_DamageInfo` 20.0 "NewEnumerator3" "NewEnumerator1"))))

(event `Death`
  (bind _mesh (`self.Mesh`))
  (`PrimitiveComponent.SetSimulatePhysics` _mesh true)
  (`PrimitiveComponent.SetCollisionEnabled` _mesh "QueryAndPhysics"))

(event `DamageResponse`
  (params (DamageResponse :type Byte :default 0))
  (`KismetSystemLibrary.PrintString` (`KismetStringLibrary.Conv_ByteToString` DamageResponse)))

(event `self.ReceiveAnyDamage`
  (params (Damage :type "Float (single-precision)") (DamageType :type "DamageType Object Reference") (InstigatedBy :type "Controller Object Reference") (DamageCauser :type "Actor Object Reference"))
  (`self.PlayAnimMontage` "/Game/HitImpact_Montage.HitImpact_Montage"))

(fn `GetCurrentHealth`
  (returns (CurrentHealth :type "Float (double-precision)"))
  (return (`/Game/Blueprints/Components/BPC_DamageSystem.Health` (`self.BPC_DamageSystem`))))

(fn `GetMaxHealth`
  (returns (MaxHealth :type "Float (double-precision)"))
  (return (`/Game/Blueprints/Components/BPC_DamageSystem.MaxHealth` (`self.BPC_DamageSystem`))))

(fn `Heal`
  (params (Amount :type "Float (double-precision)"))
  (returns (NewHealth :type "Float (double-precision)"))
  (bind _newhealth (`/Game/Blueprints/Interfaces/I_Damageable.Heal` Amount))
  (return _newhealth))

(fn `TakeDamage`
  (params (DamageInfo :type "/Game/Blueprints/Structures/S_DamageInfo Structure"))
  (returns (WasDamaged :type Boolean))
  (return false))

(fn `UserConstructionScript`
  (bind _bpc_damagesystem (`self.BPC_DamageSystem`))
  (add `/Game/Blueprints/Components/BPC_DamageSystem.OnDeath` _bpc_damagesystem (`|CreateDelegate` :!event `Death`))
  (add `/Game/Blueprints/Components/BPC_DamageSystem.OnDamageResponse` _bpc_damagesystem (`|CreateDelegate` :!event `DamageResponse`)))