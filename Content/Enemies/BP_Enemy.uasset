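; BP_Enemy is an enemy that attacks automatically on a repeating timer started at BeginPlay.
; Each attack runs a short sphere trace for Pawn objects along its forward vector, with debug drawing left on.
; On a hit, it sends a TakeDamage message to the hit actor with a damage info struct carrying a fixed amount, type and response.
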(event `self.ReceiveBeginPlay`
  (`KismetSystemLibrary.K2_SetTimerDelegate` (delegate `Attack`) 2.0 true))

(event `Attack`
  (bind _returnvalue (`self.K2_GetActorLocation`))
  (bind (_outhit _returnvalue_2) (`KismetSystemLibrary.SphereTraceSingleForObjects` :`Start` _returnvalue :`End` (+ _returnvalue (* (`self.GetActorForwardVector`) 100.0)) :`Radius` 20.0 :`ObjectTypes` (`|MakeArray` "ObjectTypeQuery3" :!type "EObjectTypeQuery Enum") :`DrawDebugType` "ForDuration" :`DrawTime` 2.0))
  (if _returnvalue_2
    (message `/Game/DamageSystem/BPI_Damageable.TakeDamage` (`.HitActor` (`GameplayStatics.BreakHitResult` _outhit)) (make `/Game/DamageSystem/S_DamageInfo` 20.0 "NewEnumerator3" "NewEnumerator1"))))

(fn `UserConstructionScript`)