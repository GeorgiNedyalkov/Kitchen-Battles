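; Base enemy projectile actor that flies at a configurable speed and gravity, with optional homing on a target, and expires after a short lifetime.
; The construction script configures projectile movement, while RotateToTarget can redirect velocity toward the target.
; On a box hit it broadcasts OnProjectileImpact, applies fixed damage, plays impact effect and sound, then destroys itself.
; An unconnected field-system snippet for breaking objects never runs.
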(event `self.ReceiveBeginPlay`
  ;[0.002428 0.002428 0.002428] Event Begin Play
  (`KismetSystemLibrary.Delay` 4.0)
  (`self.K2_DestroyActor`))

(event `RotateToTarget`
  ;[0.002428 0.002428 0.002428] Rotate to Target
  (set `MovementComponent.Velocity` (* (`KismetMathLibrary.GetDirectionUnitVector` (`self.K2_GetActorLocation`) (`self.K2_GetActorLocation` (`self.Target`))) (`self.Speed`)) (`self.ProjectileMovement`)))

(event `self.Box.OnComponentHit`
  (params (HitComponent :type "PrimitiveComponent Object Reference") (OtherActor :type "Actor Object Reference") (OtherComp :type "PrimitiveComponent Object Reference") (NormalImpulse :type "Vector Structure") (Hit :type "HitResult Structure (by ref)"))
  (bind (_bblockinghit _binitialoverlap _time _distance _location _impactpoint _normal _impactnormal _physmat _hitactor) (`GameplayStatics.BreakHitResult` Hit))
  ;[0.002428 0.002428 0.002428] Event On Hit
  (`self.OnProjectileImpact` OtherActor Hit)
  (`GameplayStatics.ApplyDamage` _hitactor 10.0)
  (`GameplayStatics.SpawnEmitterAtLocation` (`self.ImactEffect`) _location)
  (`GameplayStatics.PlaySoundAtLocation` (`self.ImpactSound`) _location (struct) 1.0 1.0 0.0 null null null null)
  (`self.K2_DestroyActor`))

(fn `UserConstructionScript`
  (bind _speed (`self.Speed`))
  (bind _projectilemovement (`self.ProjectileMovement`))
  (set `ProjectileMovementComponent.InitialSpeed` _speed _projectilemovement)
  (set `ProjectileMovementComponent.MaxSpeed` _speed _projectilemovement)
  (set `ProjectileMovementComponent.ProjectileGravityScale` (`self.Gravity`) _projectilemovement)
  (`self.Target`
    (:`then`
      (if (`self.bIsHoming`)
        (set `ProjectileMovementComponent.bIsHomingProjectile` true _projectilemovement)
        (set `ProjectileMovementComponent.HomingTargetComponent` (`Actor.RootComponent` (`self.Target`)) _projectilemovement)))
    (:`else`)))