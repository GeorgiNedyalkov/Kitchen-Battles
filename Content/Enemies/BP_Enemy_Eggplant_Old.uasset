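; BP_Enemy_Eggplant_Old is an eggplant enemy Blueprint exposing damage and health functions, with BeginPlay and construction deferring to its parent.
; Max and current health read from BPCDamageSystem, and Heal passes the amount to a Heal call and returns its result.
; TakeDamage and GetHealthPercentage are stubs that always return false and zero, so this class applies no damage through that function.
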(event `self.ReceiveBeginPlay`
  (`parent.ReceiveBeginPlay`))

(fn `GetCurrentHealth`
  (returns (CurrentHealth :type "Float (double-precision)"))
  (return (`/Game/Blueprints/Components/BPC_DamageSystem.Health` (`self.BPC_DamageSystem`))))

(fn `GetHealthPercentage`
  (returns (HealthPercentage :type "Float (double-precision)"))
  (return 0.0))

(fn `GetMaxHealth`
  (returns (MaxHealth :type "Float (double-precision)"))
  (return (`/Game/Blueprints/Components/BPC_DamageSystem.MaxHealth` (`self.BPC_DamageSystem`))))

(fn `Heal`
  (params (Amount :type "Float (double-precision)"))
  (returns (NewHealth :type "Float (double-precision)"))
  (bind _newhealth (`/Game/Blueprints/Interfaces/I_Damageable.Heal` Amount))
  (return _newhealth))

(fn `TakeDamage`
  (params (DamageInfo :type "/Game/Blueprints/Structures/S_DamageInfo Structure"))
  (returns (WasDamaged :type Boolean))
  (return false))

(fn `UserConstructionScript`
  (`parent.UserConstructionScript`))