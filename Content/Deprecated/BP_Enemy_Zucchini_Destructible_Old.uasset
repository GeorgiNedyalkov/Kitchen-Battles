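; Deprecated destructible zucchini enemy Blueprint that breaks apart when its health runs out.
; Any damage lowers a clamped HP value and prints it as debug output.
; At zero HP it enables physics simulation on a Geometry Collection and destroys the HP bar, cucumber LOD component and capsule, while the actor itself remains.
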(event `self.ReceiveAnyDamage`
  (params (Damage :type "Float (single-precision)") (DamageType :type "DamageType Object Reference") (InstigatedBy :type "Controller Object Reference") (DamageCauser :type "Actor Object Reference"))
  (bind _output_get (set `self.HP` (`KismetMathLibrary.FClamp` (- (`self.HP`) Damage) 0.0 200.0)))
  (`KismetSystemLibrary.PrintString` (`KismetStringLibrary.Conv_DoubleToString` _output_get))
  (if (<= (`self.HP`) 0.0)
    (`PrimitiveComponent.SetSimulatePhysics` (`self.GeometryCollection`) true)
    (`ActorComponent.K2_DestroyComponent` (`self.HP_bar`))
    (`ActorComponent.K2_DestroyComponent` (`self.S_Cucumber_tl2leafjw_lod3`))
    (`ActorComponent.K2_DestroyComponent` (`self.CapsuleComponent`))))

(fn `UserConstructionScript`)