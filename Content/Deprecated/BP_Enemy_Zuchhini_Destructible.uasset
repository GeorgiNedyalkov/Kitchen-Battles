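; Deprecated destructible zucchini enemy that shoots projectiles targeting the player, built on a parent class that provides base BeginPlay and Death logic.
; BeginPlay caches the first player pawn as the target.
; Shoot spawns a projectile just offset from ShootPoint, passing it that target plus an explosion effect and impact sound.
; Death enables physics simulation on the GCZuchhini component, apparently a geometry collection, and destroys the capsule.
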(event `self.ReceiveBeginPlay`
  (`parent.ReceiveBeginPlay`)
  (set `self.Target` (`GameplayStatics.GetPlayerPawn` 0)))

(event `Shoot`
  (bind (_returnvalue_location _returnvalue_rotation _returnvalue_scale) (`KismetMathLibrary.BreakTransform` (`SceneComponent.K2_GetComponentToWorld` (`self.ShootPoint`))))
  (`|SpawnActorFromClass` (`self.Projectile`) (`KismetMathLibrary.MakeTransform` (+ _returnvalue_location (20.0 0.0 0.0)) _returnvalue_rotation _returnvalue_scale) "Undefined" "MultiplyWithRoot" self 1000.0 0.0 false "/Game/StarterContent/Particles/P_Explosion.P_Explosion" "/Engine/VREditor/Sounds/UI/Camera_Shutter.Camera_Shutter" 0.0 (`self.Target`) null))

(event `self.Death`
  (`parent.Death`)
  (`PrimitiveComponent.SetSimulatePhysics` (`self.GC_Zuchhini`) true)
  (`ActorComponent.K2_DestroyComponent` (`self.CapsuleComponent`)))

(fn `UserConstructionScript`
  (`parent.UserConstructionScript`))